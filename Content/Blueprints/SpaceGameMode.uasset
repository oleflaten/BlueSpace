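; Game mode for a space game that spawns the enemy handler and declares a win when no enemies remain.
; On BeginPlay it spawns EnemyHandler_BP at a fixed location and caches its enemy count.
; Tick polls that count every frame and calls Win on BigText for as long as it is zero or below.
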(event `self.ReceiveBeginPlay`
  (bind _returnvalue (`|SpawnActorFromClass` "/Game/Blueprints/EnemyHandler_BP.EnemyHandler_BP_C" (`KismetMathLibrary.MakeTransform` (0.0 -440.0 30.0)) "AdjustIfPossibleButAlwaysSpawn" "OverrideRootScale" null null))
  (bind _output_get (set `self.EnemyHandler` _returnvalue))
  (set `self.EnemyCount` (`/Game/Blueprints/EnemyHandler_BP.EnemyCount` _output_get)))

(event `self.ReceiveTick`
  (params (DeltaSeconds :type "Float (single-precision)"))
  (bind _output_get (set `self.EnemyCount` (`/Game/Blueprints/EnemyHandler_BP.EnemyCount` (`self.EnemyHandler`))))
  (if (<= _output_get 0)
    (`/Game/Blueprints/StartWinLooseText.Win` (`self.BigText`))))

(fn `UserConstructionScript`)