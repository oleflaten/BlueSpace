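; EnemyHandler_BP spawns and drives a formation of Enemy_BP actors.
; BeginPlay spawns rows of five enemies at offsets from its own location, stepping along X up to a fixed limit, and stores them in EnemyArray.
; Each Tick moves living enemies along X by EnemySpeed scaled by delta time.
; The same loop destroys enemies flagged Killed, removes them from the array and updates EnemyCount.
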(event `self.ReceiveBeginPlay`
  ;[1 1 1] Spawn enemy grid
  (for _index (range 1 6) :!label _label
    (bind _returnvalue (`|SpawnActorFromClass` "/Game/Blueprints/Enemy_BP.Enemy_BP_C" (`KismetMathLibrary.MakeTransform` (+ (`KismetMathLibrary.MakeVector` (stale _output_get_2) (* _index (`self.Yoffset`))) (`self.K2_GetActorLocation`))) "Undefined" "OverrideRootScale" null null))
    (bind _returnvalue_2 (`KismetArrayLibrary.Array_Add` (`self.EnemyArray`) _returnvalue))
    (bind _output_get (set `self.EnemyCount` _returnvalue_2))
    (`KismetSystemLibrary.PrintString` (`KismetStringLibrary.Conv_IntToString` _output_get)))
  (bind _output_get_2 (set `self.TempXoffset` (+ (stale _output_get_2) (`self.Xoffset`))))
  (`/Engine/EditorBlueprintResources/StandardMacros.CompareFloat` _output_get_2 700.0
    (:`<`
      (goto _label))))

(event `self.ReceiveTick`
  (params (DeltaSeconds :type "Float (single-precision)"))
  (for (_array_element _array_index) (`self.EnemyArray`)
    (if (`/Game/Blueprints/Enemy_BP.Killed` _array_element)
      (`self.K2_DestroyActor` _array_element)
      (`KismetArrayLibrary.Array_Remove` (`self.EnemyArray`) _array_index)
      (set `self.EnemyCount` (`KismetArrayLibrary.Array_Length` (`self.EnemyArray`)))
      (else
        (`self.K2_SetActorLocation` _array_element (+ (`KismetMathLibrary.MakeVector` (* (`self.EnemySpeed`) DeltaSeconds)) (`self.K2_GetActorLocation` _array_element)) false false)))))

(fn `UserConstructionScript`)