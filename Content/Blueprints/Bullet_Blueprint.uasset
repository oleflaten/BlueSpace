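; Projectile actor that flies in a straight line along world X and explodes on contact with enemies.
; Tick moves it by Speed scaled by delta time, without sweep, and destroys it once its X reaches PointForDeletion.
; Overlapping an Enemy_BP or child class plays an explosion sound and particle effect, then destroys the bullet itself; the enemy is not destroyed here.
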(event `self.ReceiveActorBeginOverlap`
  (params (OtherActor :type "Actor Object Reference"))
  ;[1 1 1] Delete enemy if hit
  (if (`KismetMathLibrary.ClassIsChildOf` (`GameplayStatics.GetObjectClass` OtherActor) "/Game/Blueprints/Enemy_BP.Enemy_BP_C")
    (`GameplayStatics.PlaySound2D` "/Game/Sound/Explosion.Explosion")
    (`GameplayStatics.SpawnEmitterAtLocation` "/Game/Particles/P_Explosion.P_Explosion" (`self.K2_GetActorLocation`))
    (`self.K2_DestroyActor`)))

(event `self.ReceiveTick`
  (params (DeltaSeconds :type "Float (single-precision)"))
  (bind _returnvalue (`self.K2_GetActorLocation`))
  ;[1 1 1] Movement
  (`self.K2_SetActorLocation` (+ (`KismetMathLibrary.MakeVector` (* DeltaSeconds (`self.Speed`))) _returnvalue))
  (if (>= (.x _returnvalue) (`self.PointForDeletion`))
    (`self.K2_DestroyActor`)))

(fn `UserConstructionScript`)