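; Actor that shows the large start, win and lose messages in the space game through a TextRender component.
; On BeginPlay it displays the start text, sets a short timer to hide it, and registers itself as BigText on SpaceGameMode.
; Its Win and Loose events swap in the matching result text and make it visible again.
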(event `self.ReceiveBeginPlay`
  ;[1 1 1] Start text and set reference in GameMode
  (`TextRenderComponent.K2_SetText` (`self.TextRender`) (`self.Start`))
  (`KismetSystemLibrary.K2_SetTimer` null "HideText" 2.0)
  (bind _asspace_game_mode (cast `/Game/Blueprints/SpaceGameMode` (`GameplayStatics.GetGameMode`)))
  (set `/Game/Blueprints/SpaceGameMode.BigText` self _asspace_game_mode))

(event `Win`
  (bind _textrender (`self.TextRender`))
  ;[1 1 1] Set text if Win / Loose
  (`TextRenderComponent.K2_SetText` _textrender (`self.You Won!`))
  (`SceneComponent.SetVisibility` _textrender true false :!label _label))

(event `Loose`
  ;[1 1 1] Set text if Win / Loose
  (`TextRenderComponent.K2_SetText` (`self.TextRender`) (`self.You Lost`))
  (goto _label))

(fn `HideText`
  (`SceneComponent.SetVisibility` (`self.TextRender`) false false))

(fn `UserConstructionScript`)