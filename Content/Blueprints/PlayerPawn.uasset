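; Player pawn that moves along world axes and fires bullets.
; On BeginPlay it adds the HUD widget to the viewport and switches the player's view to the Camera target.
; Movement axis inputs offset the location directly on X and Y, scaled by Speed and delta time, without sweep collision.
; Shoot plays a laser sound, spawns Bullet_Blueprint at the pawn's transform and decrements Ammo without checking how much remains.
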(event `self.ReceiveBeginPlay`
  ;[1 1 1] Set Camera and HUD
  (bind _returnvalue (`|CreateWidget` "/Game/Blueprints/HUD_BP.HUD_BP_C"))
  (bind _output_get (set `self.HUD` _returnvalue))
  (`UserWidget.AddToViewport` _output_get 0)
  (`PlayerController.SetViewTargetWithBlend` (`GameplayStatics.GetPlayerController` 0) (`self.Camera`) 0.0 "VTBlend_Linear" 0.0 false))

(event `InputAxis|MoveForward`
  (params (AxisValue :type "Float (single-precision)"))
  ;[1 1 1] Movement
  (`self.K2_SetActorLocation` (+ (`KismetMathLibrary.MakeVector` (* (* AxisValue (`self.Speed`)) (stale `self.ReceiveTick` DeltaSeconds))) (`self.K2_GetActorLocation`))))

(event `self.ReceiveTick`
  (params (DeltaSeconds :type "Float (single-precision)"))
  ;[1 1 1] Movement
)

(event `InputAxis|MoveRight`
  (params (AxisValue :type "Float (single-precision)"))
  ;[1 1 1] Movement
  (`self.K2_SetActorLocation` (+ (`KismetMathLibrary.MakeVector` 0.0 (* (stale `self.ReceiveTick` DeltaSeconds) (* AxisValue (`self.Speed`)))) (`self.K2_GetActorLocation`))))

(event `InputAction|Shoot`
  (params (Key :type "Key Structure"))
  ;[1 1 1] Shooting
  (:`Pressed`
    (`GameplayStatics.PlaySoundAtLocation` "/Game/Sound/Laser_Shoot.Laser_Shoot" (`self.K2_GetActorLocation`))
    (`|SpawnActorFromClass` "/Game/Blueprints/Bullet_Blueprint.Bullet_Blueprint_C" (`self.GetTransform`) "Undefined" "OverrideRootScale" null null)
    (set `self.Ammo` (- (`self.Ammo`) 1))))

(fn `UserConstructionScript`)